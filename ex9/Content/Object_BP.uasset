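; Object_BP is an actor that randomly recolors its static mesh during play.
; Its construction script creates a dynamic material instance from the Material variable on the mesh's first slot.
; Tick sets the Color parameter to random RGB when game time lands near a whole second, a frame-dependent modulo check rather than a timer.
; BeginPlay prints the parent material's name, and the overlap event is empty.
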(event EventBeginPlay
  (Development|PrintString (Utilities|GetObjectName (Variables|/Script/Engine.MaterialInstance|GetParent (Variables|Default|GetDynamicMaterial)))))

(event Collision|EventActorBeginOverlap
  (params (OtherActor :type Actor%20Object%20Reference)))

(event EventTick
  (params (DeltaSeconds :type Float%20%28single-precision%29))
  (if (Math|Float|NearlyEqual(Float) (Math|Float|%(Float) (Utilities|Time|GetGameTimeinSeconds) 1.0) 0.0 0.01)
    (Rendering|Material|SetVectorParameterValue (Variables|Default|GetDynamicMaterial) "Color" (Utilities|Struct|MakeLinearColor (Math|Random|RandomFloat) (Math|Random|RandomFloat) (Math|Random|RandomFloat) 0.0) :!class /Script/Engine.MaterialInstanceDynamic)))

(fn ConstructionScript
  (bind _returnvalue (Rendering|Material|CreateDynamicMaterialInstance (Variables|Default|GetStaticMesh) 0 (Variables|Default|GetMaterial) :!class /Script/Engine.PrimitiveComponent))
  (Variables|Default|SetDynamicMaterial _returnvalue))