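; TimerTrigger is a placeable trigger actor that marks either the start or the end of a timed level run, chosen by TriggerType.
; When the player overlaps a start trigger, it records the game time in MyGameStateBase.
; An end trigger shows the FinalScreen widget with NextLevel, switches to UI input and pauses the game.
; Every instance also updates the game state's timer on Tick, regardless of type.
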(event EventBeginPlay)

(event Collision|EventActorBeginOverlap
  (params (OtherActor :type Actor%20Object%20Reference))
  (bind _returnvalue (Game|GetPlayerController 0))
  (bind _returnvalue_2 (Game|GetPlayerCharacter 0))
  (bind _returnvalue_3 (== OtherActor _returnvalue_2))
  (switch Utilities|FlowControl|Switch|SwitchonTriggerTypes (Variables|Default|GetTriggerType)
    (:NewEnumerator0
      (if _returnvalue_3
        (bind _asmy_game_state_base (Utilities|Casting|CastToMyGameStateBase (Game|GetGameState)))
        (Class|MyGameStateBase|SetStartTime _asmy_game_state_base (Utilities|Time|GetGameTimeinSeconds))))
    (:NewEnumerator1
      (if _returnvalue_3
        (bind _returnvalue_4 (UserInterface|CreateWidget "/Game/UI/FinalScreen.FinalScreen_C" _returnvalue))
        (Variables|/Game/UI/FinalScreen.FinalScreen_C|SetLevel _returnvalue_4 (Variables|Default|GetNextLevel))
        (UserInterface|Viewport|AddtoViewport _returnvalue_4 0)
        (Input|SetInputModeUIOnly _returnvalue _returnvalue_4 "DoNotLock")
        (Variables|/Script/Engine.PlayerController|SetbShowMouseCursor _returnvalue true)
        (Game|SetGamePaused true)))))

(event EventTick
  (params (DeltaSeconds :type Float%20%28single-precision%29))
  (bind _asmy_game_state_base (Utilities|Casting|CastToMyGameStateBase (Game|GetGameState)))
  (Class|MyGameStateBase|UpdateTimer _asmy_game_state_base (Utilities|Time|GetGameTimeinSeconds)))

(fn ConstructionScript)