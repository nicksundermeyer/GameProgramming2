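; BP_BasicEnemyPawn is an enemy pawn Blueprint with two AI movement behaviors, chasing the player and patrolling points.
; ChasePlayer uses AIMoveTo toward the first player's pawn and re-calls itself on success.
; Patrol moves through PatrolPoints and repeats on success, but its wrap check lets the index run past the array end.
; The switch choosing between behaviors is unconnected and BeginPlay is empty, so nothing here starts either loop.
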(event Custom|ChasePlayer
  (AI|AIMoveTo self "0, 0, 0" (Game|Player|GetPlayerPawn 0) 5.0 false
    (:OnSuccess
      (CallFunction|ChasePlayer))))

(event Custom|Patrol
  (AI|AIMoveTo self "0, 0, 0" (Utilities|Array|Get(acopy) (Variables|Default|GetpatrolPoints) (Variables|Default|GetcurrentPatrolPoint)) 5.0 false
    (:OnSuccess
      (if (> (Variables|Default|GetcurrentPatrolPoint) (Utilities|Array|Length (Variables|Default|GetpatrolPoints)))
        (Variables|Default|SetcurrentPatrolPoint 0)
        (else
          (Variables|Default|SetcurrentPatrolPoint (+ (Variables|Default|GetcurrentPatrolPoint) 1))))
      (CallFunction|Patrol))))

(event EventBeginPlay)

(event Collision|EventActorBeginOverlap
  (params (OtherActor :type Actor%20Object%20Reference)))

(event EventTick
  (params (DeltaSeconds :type Float%20%28single-precision%29)))

(fn ConstructionScript)