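; BP_EnemyAIPatrol is an enemy character that walks a looping route through assigned patrol point actors.
; On BeginPlay it sets its movement component's max walk speed from WalkSpeed, then starts patrolling.
; Patrol uses AIMoveTo toward the current point and, on success, advances the index, wraps to the first, and calls itself again.
; A failed move has no handler, so the patrol stops there.
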(event Custom|Patrol
  ;[1 1 1] Patrol Points
  (AI|AIMoveTo self "0, 0, 0" (Utilities|Array|Get(acopy) (Variables|Default|GetpatrolPoints) (Variables|Default|GetcurrentPatrolPoint)) 5.0 false
    (:OnSuccess
      (Variables|Default|SetcurrentPatrolPoint (+ (Variables|Default|GetcurrentPatrolPoint) 1))
      (if (> (Variables|Default|GetcurrentPatrolPoint) (- (Utilities|Array|Length (Variables|Default|GetpatrolPoints)) 1))
        (Variables|Default|SetcurrentPatrolPoint 0))
      (CallFunction|Patrol))))

(event EventBeginPlay
  (bind _ascharacter_movement_component (Utilities|Casting|CastToCharacterMovementComponent (Pawn|GetMovementComponent)))
  (Variables|/Script/Engine.CharacterMovementComponent|SetMaxWalkSpeed _ascharacter_movement_component (Variables|Default|GetwalkSpeed))
  (CallFunction|Patrol))

(fn ConstructionScript)