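; BP_EnemyAICharacter is an enemy character that either chases the player or patrols a set of points.
; BeginPlay applies WalkSpeed to the movement component, then picks the behavior from AIState once, with no later switching shown.
; Both behaviors re-issue AI MoveTo on success, with patrol cycling through PatrolPoints in a loop.
; Failed moves are not handled, so a failure ends the active behavior.
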(event Custom|Patrol
  ;[1 1 1] Patrol Points
  (AI|AIMoveTo self "0, 0, 0" (Utilities|Array|Get(acopy) (Variables|Default|GetpatrolPoints) (Variables|Default|GetcurrentPatrolPoint)) 5.0 false
    (:OnSuccess
      (Variables|Default|SetcurrentPatrolPoint (+ (Variables|Default|GetcurrentPatrolPoint) 1))
      (if (> (Variables|Default|GetcurrentPatrolPoint) (- (Utilities|Array|Length (Variables|Default|GetpatrolPoints)) 1))
        (Variables|Default|SetcurrentPatrolPoint 0))
      (CallFunction|Patrol))))

(event Custom|ChasePlayer
  ;[1 1 1] Chase Player
  (AI|AIMoveTo self "0, 0, 0" (Game|Player|GetPlayerPawn 0) 5.0 false
    (:OnSuccess
      (CallFunction|ChasePlayer))))

(event EventTick
  (params (DeltaSeconds :type Float%20%28single-precision%29)))

(event EventBeginPlay
  ;[1 1 1] Setting walk speed
  (bind _ascharacter_movement_component (Utilities|Casting|CastToCharacterMovementComponent (Pawn|GetMovementComponent)))
  (Variables|/Script/Engine.CharacterMovementComponent|SetMaxWalkSpeed _ascharacter_movement_component (Variables|Default|GetwalkSpeed))
  ;[1 1 1] Set AI Behavior
  (switch Utilities|FlowControl|Switch|SwitchonEAIState (Variables|Default|GetAIState)
    (:NewEnumerator0
      (CallFunction|ChasePlayer))
    (:NewEnumerator1
      (CallFunction|Patrol))))

(fn ConstructionScript)