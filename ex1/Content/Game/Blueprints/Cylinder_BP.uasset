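; Cylinder Blueprint that moves itself through a looping list of waypoints, beginning from its location at BeginPlay.
; Each Tick advances a normalized alpha by Speed times delta time and sets the location interpolated between the segment start and current waypoint.
; On reaching a waypoint, it becomes the new start, the alpha resets and the index wraps by modulo.
; Speed is a fraction of a segment per second, independent of distance.
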(event EventBeginPlay
  ;[1 1 1] Initialize with starting actor location
  (Variables|Default|SetStartingLocation (Transformation|GetActorLocation)))

(event Collision|EventActorBeginOverlap
  (params (OtherActor :type Actor%20Object%20Reference)))

(event EventTick
  (params (DeltaSeconds :type Float%20%28single-precision%29))
  (if (CallFunction|AtWaypoint? (Transformation|GetActorLocation))
    (CallFunction|SetNextWaypoint)
    (else
      (bind _nextlocation (CallFunction|GetNextLocation "0, 0, 0" DeltaSeconds))
      (Transformation|SetActorLocation _nextlocation false false))))

(fn ConstructionScript)

(fn AtWaypoint?
  (params (CurrentLocation :type Vector))
  (return (Math|Vector|Equal(Vector) CurrentLocation (Utilities|Array|Get(acopy) (Variables|Default|GetWaypoints) (Variables|Default|GetCurrentIndex)) 0.0001)))

(fn SetNextWaypoint
  (Variables|Default|SetStartingLocation (Utilities|Array|Get(acopy) (Variables|Default|GetWaypoints) (Variables|Default|GetCurrentIndex)))
  (Variables|Default|SetCurrentIndex (Math|Integer|%(Integer) (+ (Variables|Default|GetCurrentIndex) 1) (Utilities|Array|Length (Variables|Default|GetWaypoints))))
  (Variables|Default|SetInterpBy 0.0))

(fn GetNextLocation
  (params (CurrentLocation :type Vector) (DeltaTime :type Float%20%28single-precision%29))
  (bind _output_get (Variables|Default|SetInterpBy (+ (Variables|Default|GetInterpBy) (* (Variables|Default|GetSpeed) DeltaTime))))
  (return (CallFunction|Interpolate (Variables|Default|GetStartingLocation) (Utilities|Array|Get(acopy) (Variables|Default|GetWaypoints) (Variables|Default|GetCurrentIndex)) _output_get)))