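; Movement Blueprint that spins its actor while sliding it back and forth around its starting location.
; BeginPlay stores the initial location, then each Tick adds DeltaRotate to the rotation and DeltaMove times Delta to the location.
; Delta flips sign whenever distance from the start exceeds MaxDistance, reversing travel.
; Steps are per frame without delta-time scaling, and each transform update forces unit scale without sweeping.
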(event EventBeginPlay
  (Variables|Default|SetInitialPosition (Transformation|GetActorLocation)))

(event Collision|EventActorBeginOverlap
  (params (OtherActor :type Actor%20Object%20Reference)))

(event EventTick
  (params (DeltaSeconds :type Float%20%28single-precision%29))
  (bind _returnvalue (Transformation|GetActorRotation))
  (bind _deltarotate (Variables|Default|GetDeltaRotate))
  (bind (_roll _pitch _yaw) (Math|Rotator|BreakRotator _returnvalue))
  (bind (_x _y _z) (Math|Vector|BreakVector _deltarotate))
  (Transformation|SetActorTransform (Math|Transform|MakeTransform (+ (Transformation|GetActorLocation) (* (Variables|Default|GetDeltaMove) (Variables|Default|GetDelta))) (Math|Rotator|MakeRotator (+ _roll _x) (+ _pitch _y) (+ _z _yaw))))
  (if (> (Math|Vector|VectorLength (- (Transformation|GetActorLocation) (Variables|Default|GetInitialPosition))) (Variables|Default|GetMaxDistance))
    (Variables|Default|SetDelta (* (Variables|Default|GetDelta) -1.0))))

(fn ConstructionScript)